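; Target dummy that reacts physically to hits and spawns floating damage text at its head when its health component reports damage.
; Point damage on any bone but the pelvis simulates physics below that bone, applies an impulse, and blends back to animation via a timeline.
; Radial damage ragdolls the whole mesh, then after a delay a stand-up timeline blends physics out and re-aligns the mesh to the capsule.
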(event `self.TPS_Health.OnDamageReceived`
  (params (DamagedActor :type "Actor Object Reference") (Damage :type "Float (single-precision)") (DamageType :type "DamageType Object Reference") (InstigatedBy :type "Controller Object Reference") (DamageCauser :type "Actor Object Reference"))
  (`|SpawnActorFromClass` "/Game/Core/Targets/BP_DamageText.BP_DamageText_C" (`KismetMathLibrary.MakeTransform` (`SceneComponent.GetSocketLocation` (`self.SkeletalMesh`) "head")) "Undefined" "OverrideRootScale" DamageCauser (`KismetTextLibrary.Conv_DoubleToText` Damage "HalfToEven") null))

(event `self.ReceivePointDamage`
  (params (Damage :type "Float (single-precision)") (DamageType :type "DamageType Object Reference") (HitLocation :type "Vector Structure") (HitNormal :type "Vector Structure") (HitComponent :type "PrimitiveComponent Object Reference") (BoneName :type Name) (ShotFromDirection :type "Vector Structure") (InstigatedBy :type "Controller Object Reference") (DamageCauser :type "Actor Object Reference") (HitInfo :type "HitResult Structure (by ref)"))
  (bind _skeletalmesh (`self.SkeletalMesh`))
  (bind (_hitinfo_bblockinghit _hitinfo_binitialoverlap _hitinfo_time _hitinfo_distance _hitinfo_location _hitinfo_impactpoint _hitinfo_normal _hitinfo_impactnormal _hitinfo_physmat _hitinfo_hitactor _hitinfo_hitcomponent _hitinfo_hitbonename) (`GameplayStatics.BreakHitResult` (`self.HitInfo`)))
  (if (!= BoneName "pelvis")
    (bind _output_get (set `self.HitBone` BoneName))
    (set `self.HitInfo` HitInfo)
    (`SkeletalMeshComponent.SetAllBodiesBelowSimulatePhysics` (`self.SkeletalMesh`) _output_get true true)
    (`SkeletalMeshComponent.SetEnablePhysicsBlending` (`self.SkeletalMesh`) true)
    (`SkeletalMeshComponent.SetAllBodiesBelowPhysicsBlendWeight` (`self.SkeletalMesh`) (`self.HitBone`) 0.5 false true)
    (`PrimitiveComponent.AddImpulseAtLocation` (`self.SkeletalMesh`) (* _hitinfo_impactnormal -10000.0) _hitinfo_impactpoint _hitinfo_hitbonename)
    (bind (_direction _newtrack_0) (`Timeline|HitReaction` :!via `PlayFromStart`)
      (:`Update`
        (`SkeletalMeshComponent.SetAllBodiesBelowPhysicsBlendWeight` (`self.SkeletalMesh`) (`self.HitBone`) _newtrack_0 false true))
      (:`Finished`
        (`SkeletalMeshComponent.SetAllBodiesPhysicsBlendWeight` (`self.SkeletalMesh`) 0.0 false)
        (`SkeletalMeshComponent.SetEnablePhysicsBlending` _skeletalmesh false)
        (`SkeletalMeshComponent.SetAllBodiesSimulatePhysics` _skeletalmesh false)))))

(event `self.ReceiveRadialDamage`
  (params (DamageReceived :type "Float (single-precision)") (DamageType :type "DamageType Object Reference") (Origin :type "Vector Structure") (HitInfo :type "HitResult Structure (by ref)") (InstigatedBy :type "Controller Object Reference") (DamageCauser :type "Actor Object Reference"))
  (bind _skeletalmesh (`self.SkeletalMesh`))
  (bind (_returnvalue_location _returnvalue_rotation) (`KismetMathLibrary.BreakTransform` (`SceneComponent.K2_GetComponentToWorld` (`self.Capsule`))))
  (`SkeletalMeshComponent.SetAllBodiesSimulatePhysics` (`self.SkeletalMesh`) true)
  (`SkeletalMeshComponent.SetEnablePhysicsBlending` (`self.SkeletalMesh`) false)
  (`SkeletalMeshComponent.SetAllBodiesPhysicsBlendWeight` (`self.SkeletalMesh`) 1.0 false)
  (`KismetSystemLibrary.Delay` 1.0)
  (bind (_direction _standup) (`Timeline|Timeline_0` :!via `PlayFromStart`)
    (:`Update`
      (`SkeletalMeshComponent.SetAllBodiesPhysicsBlendWeight` (`self.SkeletalMesh`) _standup false))
    (:`Finished`
      (`SkeletalMeshComponent.SetAllBodiesPhysicsBlendWeight` (`self.SkeletalMesh`) 0.0 false)
      (`SkeletalMeshComponent.SetEnablePhysicsBlending` _skeletalmesh false)
      (`SkeletalMeshComponent.SetAllBodiesSimulatePhysics` _skeletalmesh false)
      (`SceneComponent.K2_SetWorldLocationAndRotation` (`self.SkeletalMesh`) (+ _returnvalue_location (0.0 0.0 -44.0)) _returnvalue_rotation false false))))

(fn `UserConstructionScript`)