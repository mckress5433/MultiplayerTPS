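; Destructible explosive barrel that catches fire when shot or otherwise hit by point damage, then explodes.
; Each hit attaches flame particles, and the first starts a looping timer of self-damage.
; At zero TPS_Health it clears flames and timer, then spawns an explosion with radial damage and force before a delayed destroy.
; Component fracture jumps straight to the explosion, bypassing that cleanup and its DoOnce guard.
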(event `self.ReceivePointDamage`
  (params (Damage :type "Float (single-precision)") (DamageType :type "DamageType Object Reference") (HitLocation :type "Vector Structure") (HitNormal :type "Vector Structure") (HitComponent :type "PrimitiveComponent Object Reference") (BoneName :type Name) (ShotFromDirection :type "Vector Structure") (InstigatedBy :type "Controller Object Reference") (DamageCauser :type "Actor Object Reference") (HitInfo :type "HitResult Structure (by ref)"))
  (bind _destructiblecomponent (`self.DestructibleComponent`))
  (if (not (`self.Destroyed?`))
    (bind _returnvalue (`GameplayStatics.SpawnEmitterAttached` "/Engine/Tutorial/SubEditors/TutorialAssets/TutorialParticleSystem.TutorialParticleSystem" _destructiblecomponent "None" (`KismetMathLibrary.InverseTransformLocation` (`SceneComponent.K2_GetComponentToWorld` _destructiblecomponent) HitLocation) (struct) (0.1 0.1 0.1)))
    (`KismetArrayLibrary.Array_Add` (`self.FlameParticles`) _returnvalue)
    (`/Engine/EditorBlueprintResources/StandardMacros.DoOnce` false
      (:`Completed`
        (bind _returnvalue_2 (`KismetSystemLibrary.K2_SetTimerDelegate` (delegate `DamageTimer`) 1.0 true))
        (set `self.DamageTimer_Handle` _returnvalue_2)))))

(event `DamageTimer`
  (`GameplayStatics.ApplyDamage` self 10.0))

(event `self.TPS_Health.OnHealthChanged`
  (params (HealthComp :type "TPS_HealthComponent Object Reference") (Health :type "Float (single-precision)") (HealthDelta :type "Float (single-precision)"))
  (if (<= Health 0.0)
    (`/Engine/EditorBlueprintResources/StandardMacros.DoOnce` false
      (:`Completed`
        (set `self.Destroyed?` true)
        (`KismetSystemLibrary.K2_ClearAndInvalidateTimerHandle` (`self.DamageTimer_Handle`))
        (for _array_element (`self.FlameParticles`)
          (`ActorComponent.K2_DestroyComponent` _array_element))
        (`GameplayStatics.SpawnEmitterAtLocation` "/Game/Resource/Packs/Explosions/Particles/P_ImpactExplosion7.P_ImpactExplosion7" (`SceneComponent.K2_GetComponentLocation` (`self.DestructibleComponent`)) (struct :`Pitch` 90.0) :!label _label)
        (`GameplayStatics.ApplyRadialDamage` :`BaseDamage` 200.0 :`Origin` (`SceneComponent.K2_GetComponentLocation` (`self.DestructibleComponent`)) :`DamageRadius` 200.0 :`DamageCauser` null :`InstigatedByController` null :`bDoFullDamage` true)
        (`ActorComponent.Activate` (`self.RadialForce`) false)
        (`KismetSystemLibrary.Delay` 2.0)
        (`self.K2_DestroyActor`)))))

(event `self.DestructibleComponent.OnComponentFracture`
  (params (HitPoint :type "Vector Structure (by ref)") (HitDirection :type "Vector Structure (by ref)"))
  (goto _label))

(fn `UserConstructionScript`)