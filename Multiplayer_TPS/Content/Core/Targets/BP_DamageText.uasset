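; BP_DamageText is a floating damage text actor that displays a text value in the world and then removes itself.
; On BeginPlay it writes the text variable to its TextRender and stores its spawn location.
; A timeline offsets it vertically by a Height track while rotating it toward its owner's location each update.
; The actor destroys itself when the timeline finishes.
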(event `self.ReceiveBeginPlay`
  (`TextRenderComponent.K2_SetText` (`self.TextRender`) (`self.NewVar_1`))
  (set `self.NewVar_0` (`self.K2_GetActorLocation`))
  (bind (_direction _height) (`Timeline|AnimTimeline` :!via `PlayFromStart`)
    (:`Update`
      (bind _returnvalue (+ (`self.NewVar_0`) (`KismetMathLibrary.MakeVector` 0.0 0.0 _height)))
      (`self.K2_SetActorLocationAndRotation` _returnvalue (`KismetMathLibrary.FindLookAtRotation` _returnvalue (`self.K2_GetActorLocation` (`self.GetOwner`)))))
    (:`Finished`
      (`self.K2_DestroyActor`))))

(fn `UserConstructionScript`)