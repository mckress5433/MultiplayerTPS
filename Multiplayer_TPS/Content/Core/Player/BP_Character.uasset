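; Player character Blueprint that creates the player HUD widget and toggles its key-info panel on both press and release of the KeyInfo input.
; When PawnCharacter is set, it disables input and runs two endless delay loops that randomize walk speed and trigger periodic jumps.
; Firing and reload montage events pick a sighted or hip section from IsAiming, with ReloadFinished called as the reload montage blends out.
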(event `InputAction|KeyInfo`
  (params (Key :type "Key Structure"))
  (:`Pressed`
    (`/Game/Core/Player/Widgets/WBP_Player.FlipFlopVisibleKeyInfoPanel` (`self.WBP_Player`) :!label _label))
  (:`Released`
    (goto _label)))

(event `self.ReceiveBeginPlay`
  (`parent.ReceiveBeginPlay`)
  (`|ExecutionSequence`
    (:`then_0`
      (bind _returnvalue (`|CreateWidget` "/Game/Core/Player/Widgets/WBP_Player.WBP_Player_C" (`GameplayStatics.GetPlayerController` 0)))
      (bind _output_get (set `self.WBP_Player` _returnvalue))
      (`UserWidget.AddToViewport` _output_get 0))
    (:`then_1`
      ;[0.008975 1 0] Pawn walking cycle
      (if (`self.PawnCharacter`)
        (`self.DisableInput` null)
        (`|ExecutionSequence`
          (:`then_0`
            (set `CharacterMovementComponent.MaxWalkSpeed` (`KismetMathLibrary.RandomFloatInRange` 500.0 600.0) (`self.CharacterMovement`) :!label _label_2)
            (`KismetSystemLibrary.Delay` (`KismetMathLibrary.RandomFloatInRange` 2.0 4.0))
            (goto _label_2))
          (:`then_1`
            (`KismetSystemLibrary.Delay` (`KismetMathLibrary.RandomFloatInRange` 2.0 4.0) :!label _label_3)
            (`self.Jump`)
            (`KismetSystemLibrary.Delay` 0.2)
            (`self.StopJumping`)
            (goto _label_3)))))))

(event `self.PlayFiringMontage`
  ;[1 1 1] Montages
  (`|PlayMontage` (`self.Mesh`) "/Game/Core/Player/Animations/AM_Firing.AM_Firing" 1.0 0.0 (select `bool` (`self.bIsAiming`) :`false` "RifleHip" :`true` "RifleSighted" :!type "Name")))

(event `self.PlayReloadMontage`
  ;[1 1 1] Montages
  (`|PlayMontage` (`self.Mesh`) "/Game/Core/Player/Animations/AM_Reload.AM_Reload" 1.0 0.0 (select `bool` (`self.bIsAiming`) :`false` "RifleHip" :`true` "RifleSighted" :!type "Name")
    (:`OnBlendOut`
      (`self.ReloadFinished`))))

(fn `UserConstructionScript`)